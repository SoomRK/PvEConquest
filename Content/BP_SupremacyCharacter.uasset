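; Player character for Mordhau's Supremacy mode, taking its profile and equipment from the controller's ClassMap by CharacterType.
; CharacterType gates passives such as repairing placeables, healing teammates on melee kills, damage resistances and bonus damage.
; Volley (in Hookshot-named functions), Shockwave and Immortality specials run as two-stage ability motions, storing cooldowns on the controller.
; Incoming damage chains through the attacker's ModifyOutgoingDamage; base perks apply server-side after initialization.
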(event Custom|RequestVolley
  (params (Location :type Vector))
  (CallFunction|SpecialCooldown 8e+01)
  (Utilities|Casting|CastToBP_SupremacyAbilityMotion (Class|AdvancedCharacter|GetMotion))
  (bind _returnvalue (Game|SpawnActorfromClass "/Game/Mordhau/Blueprints/GameModes/Horde/BP_VolleyArea.BP_VolleyArea_C" (Math|Transform|MakeTransform Location) "AlwaysSpawn" 0 (Pawn|GetController) 0))
  (Variables|/Game/Mordhau/Blueprints/GameModes/Horde/BP_VolleyArea.BP_VolleyArea_C|SetDamageMultiplier _returnvalue 0.7)
  (bind _returnvalue_2 (Rendering|Material|CreateDynamicMaterialInstance (Variables|/Game/Mordhau/Blueprints/GameModes/Horde/BP_VolleyArea.BP_VolleyArea_C|GetDecal _returnvalue) :!class /Script/Engine.DecalComponent))
  (if (== (Variables|Default|GetTeam) 0)
    (Rendering|Material|SetVectorParameterValue _returnvalue_2 "ColorA" "(R=0.434154,G=0.000000,B=0.000000,A=1.000000)" :!class /Script/Engine.MaterialInstanceDynamic)
    (else
      (Rendering|Material|SetVectorParameterValue _returnvalue_2 "ColorA" "(R=0.018500,G=0.063010,B=0.184475,A=1.000000)" :!class /Script/Engine.MaterialInstanceDynamic))))

(event Custom|MaintenanceTick
  (if (not (Class|AdvancedCharacter|GetIsDead))
    (if (CallFunction|IsCharacterType "NewEnumerator4")
      (bind _asbp_mordhau_player_controller (Utilities|Casting|CastToBP_MordhauPlayerController (Pawn|GetController)))
      (bind _values (Utilities|Map|Values (Variables|/Game/Mordhau/Blueprints/BP_MordhauPlayerController.BP_MordhauPlayerController_C|GetPlaceableArrays _asbp_mordhau_player_controller)))
      (for _array_element _values
        (for _array_element_2 (Utilities|Struct|BreakArrayOfActor _array_element)
          (Utilities|IsValid _array_element_2
            (:Is%20Valid
              (bind _asbp_destroyable_actor (Utilities|Casting|CastToBP_DestroyableActor _array_element_2)
                (:then
                  (if (> (Variables|/Game/Mordhau/Blueprints/Interactables/Environment/BP_DestroyableActor.BP_DestroyableActor_C|GetHealth _asbp_destroyable_actor) 0.0)
                    (Default|SetHealth _asbp_destroyable_actor (+ (Variables|/Game/Mordhau/Blueprints/Interactables/Environment/BP_DestroyableActor.BP_DestroyableActor_C|GetHealth _asbp_destroyable_actor) 1e+01))))
                (:CastFailed
                  (bind _asbp_deployable_ballista (Utilities|Casting|CastToBP_DeployableBallista _array_element_2))
                  (if (not (Class|AdvancedCharacter|GetIsDead _asbp_deployable_ballista))
                    (Class|AdvancedCharacter|OffsetHealth _asbp_deployable_ballista 10 true)))))))))))

(event Custom|TriggerImmortality
  (Variables|Default|SetIsImmortal true)
  (Variables|Default|SetbIsUnflinchable true)
  (Utilities|FlowControl|RetriggerableDelay (Variables|Default|GetLastAbilityDuration))
  (Variables|Default|SetIsImmortal false)
  (Variables|Default|SetbIsUnflinchable false))

(event EventBeginPlay
  (|CallParentFunction)
  (Utilities|FlowControl|Sequence
    (:then_0
      (if (CallFunction|IsCharacterType "NewEnumerator4")
        (bind _returnvalue (Utilities|Time|SetTimerbyEvent (delegate Custom|MaintenanceTick) 1e+01 true))
        (Variables|Default|SetMaintenanceTimer _returnvalue)))))

(event EventOnPostProfileAssigned
  (bind _profile (Variables|Default|GetProfile))
  (bind (_name _gearcustomization _appearancecustomization _facecustomization _skillscustomization _category) (Utilities|Struct|BreakCharacterProfile _profile))
  (|CallParentFunction)
  (Utilities|FlowControl|DoOnce false
    (:Completed
      (Utilities|IsValid (Game|GetGameState) :!label _label
        (:Is%20Valid
          (bind _asbp_supremacy_player_controller (Utilities|Casting|CastToBP_SupremacyPlayerController (Class|AdvancedCharacter|GetControllerIncludingVehicle)))
          (if (CallFunction|IsCharacterType "NewEnumerator8")
            (Class|MordhauCharacter|AssignProfile (Utilities|Struct|MakeCharacterProfile "Unnamed" (.GearCustomization (Utilities|Struct|BreakCharacterProfile (.Profiles (Utilities|Struct|BreakSTRUCT_ConquestClass_2 (.Value (Utilities|Map|Find (Variables|/PvEconquest/BP_SupremacyPlayerController.BP_SupremacyPlayerController_C|GetClassMap _asbp_supremacy_player_controller) (Utilities|Enum|ByteToEnumENUM_ConquestClasses (Variables|Default|GetCharacterType)))))))) (.AppearanceCustomization (Utilities|Struct|BreakCharacterProfile (.Profiles (Utilities|Struct|BreakSTRUCT_ConquestClass_2 (.Value (Utilities|Map|Find (Variables|/PvEconquest/BP_SupremacyPlayerController.BP_SupremacyPlayerController_C|GetClassMap _asbp_supremacy_player_controller) (Utilities|Enum|ByteToEnumENUM_ConquestClasses (Variables|Default|GetCharacterType)))))))) (.FaceCustomization (Utilities|Struct|BreakCharacterProfile (.Profiles (Utilities|Struct|BreakSTRUCT_ConquestClass_2 (.Value (Utilities|Map|Find (Variables|/PvEconquest/BP_SupremacyPlayerController.BP_SupremacyPlayerController_C|GetClassMap _asbp_supremacy_player_controller) (Utilities|Enum|ByteToEnumENUM_ConquestClasses (Variables|Default|GetCharacterType)))))))) (.SkillsCustomization (Utilities|Struct|BreakCharacterProfile (.Profiles (Utilities|Struct|BreakSTRUCT_ConquestClass_2 (.Value (Utilities|Map|Find (Variables|/PvEconquest/BP_SupremacyPlayerController.BP_SupremacyPlayerController_C|GetClassMap _asbp_supremacy_player_controller) (Utilities|Enum|ByteToEnumENUM_ConquestClasses (Variables|Default|GetCharacterType)))))))) (.Category (Utilities|Struct|BreakCharacterProfile (.Profiles (Utilities|Struct|BreakSTRUCT_ConquestClass_2 (.Value (Utilities|Map|Find (Variables|/PvEconquest/BP_SupremacyPlayerController.BP_SupremacyPlayerController_C|GetClassMap _asbp_supremacy_player_controller) (Utilities|Enum|ByteToEnumENUM_ConquestClasses (Variables|Default|GetCharacterType))))))))))
            (else
              (Class|MordhauCharacter|AssignProfile (Utilities|Struct|MakeCharacterProfile (.Name (Utilities|Struct|BreakCharacterProfile (.Profiles (Utilities|Struct|BreakSTRUCT_ConquestClass_2 (.Value (Utilities|Map|Find (Variables|/PvEconquest/BP_SupremacyPlayerController.BP_SupremacyPlayerController_C|GetClassMap _asbp_supremacy_player_controller) (Utilities|Enum|ByteToEnumENUM_ConquestClasses (Variables|Default|GetCharacterType)))))))) (.GearCustomization (Utilities|Struct|BreakCharacterProfile (.Profiles (Utilities|Struct|BreakSTRUCT_ConquestClass_2 (.Value (Utilities|Map|Find (Variables|/PvEconquest/BP_SupremacyPlayerController.BP_SupremacyPlayerController_C|GetClassMap _asbp_supremacy_player_controller) (Utilities|Enum|ByteToEnumENUM_ConquestClasses (Variables|Default|GetCharacterType)))))))) (.AppearanceCustomization (Utilities|Struct|BreakCharacterProfile (.Profiles (Utilities|Struct|BreakSTRUCT_ConquestClass_2 (.Value (Utilities|Map|Find (Variables|/PvEconquest/BP_SupremacyPlayerController.BP_SupremacyPlayerController_C|GetClassMap _asbp_supremacy_player_controller) (Utilities|Enum|ByteToEnumENUM_ConquestClasses (Variables|Default|GetCharacterType)))))))) _facecustomization (.SkillsCustomization (Utilities|Struct|BreakCharacterProfile (.Profiles (Utilities|Struct|BreakSTRUCT_ConquestClass_2 (.Value (Utilities|Map|Find (Variables|/PvEconquest/BP_SupremacyPlayerController.BP_SupremacyPlayerController_C|GetClassMap _asbp_supremacy_player_controller) (Utilities|Enum|ByteToEnumENUM_ConquestClasses (Variables|Default|GetCharacterType)))))))) _category))))
          (for _array_element (.Equipment (Utilities|Struct|BreakSTRUCT_ConquestClass_2 (.Value (Utilities|Map|Find (Variables|/PvEconquest/BP_SupremacyPlayerController.BP_SupremacyPlayerController_C|GetClassMap _asbp_supremacy_player_controller) (Utilities|Enum|ByteToEnumENUM_ConquestClasses (Variables|Default|GetCharacterType))))))
            (Default|GiveItem _asbp_supremacy_player_controller _array_element))
          (Class|MordhauCharacter|SwitchEquipmentbyIndex)
          (Variables|Default|SetInitialized true))
        (:Is%20Not%20Valid
          (Utilities|FlowControl|Delay 0.2)
          (goto _label))))))

(event EventTick
  (params (DeltaSeconds :type Float%20%28single-precision%29))
  (|CallParentFunction DeltaSeconds)
  (if (Variables|Default|GetInitialized)
    (Utilities|FlowControl|DoOnce false
      (:Completed
        (Utilities|FlowControl|Delay 0.3)
        (Networking|SwitchHasAuthority
          (:Authority
            (for _array_element (Variables|Default|GetBasePerks)
              (CallFunction|AssignPerks _array_element))))))))

(event EventOnKilled
  (params (EventInstigator :type Controller%20Object%20Reference))
  (|CallParentFunction EventInstigator)
  (Utilities|FlowControl|Sequence
    (:then_0
      (Networking|SwitchHasAuthority
        (:Authority
          (for _array_element (Variables|Default|GetEquipment)
            (bind _returnvalue (Class|MordhauCharacter|DropEquipment _array_element true))
            (Actor|DestroyActor _returnvalue)))))
    (:then_1
      (bind _returnvalue_2 (Class|AdvancedCharacter|GetLastNetDamageType))
      (if (Utilities|Enum|Equal(Enum) _returnvalue_2 "Melee")
        (bind _returnvalue_3 (Class|AdvancedCharacter|GetLastNetDamageSource))
        (bind _asbp_supremacy_character (Utilities|Casting|CastToBP_SupremacyCharacter _returnvalue_3))
        (CallFunction|AwardHealthonKilltoTeammates _asbp_supremacy_character)))))

(event EventOnDied
  (params (Angle :type Float%20%28single-precision%29) (Type :type EMordhauDamageType%20Enum :default "Generic") (SubType :type Byte :default 0) (Bone :type Name :default "None") (Point :type Vector :default "0, 0, 0") (Source :type Actor%20Object%20Reference) (Agent :type Actor%20Object%20Reference))
  (|CallParentFunction Angle Type SubType Bone Point Source Agent)
  (if (CallFunction|IsCharacterType "NewEnumerator4")
    (Utilities|Time|ClearandInvalidateTimerbyHandle (Variables|Default|GetMaintenanceTimer))))

(event EventOnBlockedMelee
  (params (HitResult :type Hit%20Result%20Structure%20%28by%20ref%29) (Attacker :type Mordhau%20Character%20Object%20Reference))
  (|CallParentFunction HitResult Attacker)
  (if (Class|AdvancedCharacter|GetIsDead)
    (bind _asbp_supremacy_character (Utilities|Casting|CastToBP_SupremacyCharacter Attacker))
    (if (CallFunction|IsCharacterType _asbp_supremacy_character "NewEnumerator6")
      (if (Math|Random|RandomBoolwithWeight 0.15)
        (Class|MordhauCharacter|AssignNetMotionSimple (Utilities|Enum|LiteralenumEMotionType "Stunned") 127)
        (Variables|Default|SetStunnedBySkillCounter (+ (Variables|Default|GetStunnedBySkillCounter) 1))))))

(event Input|KeyboardEvents|Divide
  (params (Key :type Key%20Structure :default "None"))
  (:Pressed
    (CallFunction|DebugCharacter (Utilities|String|Append "CharacterType=" (Utilities|String|ToString(Byte) (Variables|Default|GetCharacterType))))))

(fn ConstructionScript
  (|CallParentFunction))

(fn AwardHealthonKilltoTeammates
  (if (not (Class|AdvancedCharacter|GetIsDead))
    (if (CallFunction|IsCharacterType "NewEnumerator5")
      (bind _outactors (Actor|GetAllActorsOfClass "BP_SupremacyCharacter_C"))
      (for _array_element _outactors
        (if (and (not (Class|AdvancedCharacter|GetIsDead _array_element)) (!= _array_element self))
          (Class|AdvancedCharacter|OffsetHealth _array_element 5 true)
          (bind _asbp_mordhau_player_controller (Utilities|Casting|CastToBP_MordhauPlayerController (Class|AdvancedCharacter|GetControllerIncludingVehicle)))
          (Class|MordhauPlayerController|GiveClientScoreBP _asbp_mordhau_player_controller "Heal" 5))))))

(fn ModifyDamage
  (params (DamageAmount :type Float%20%28single-precision%29) (DamageInfo :type Mordhau%20Damage%20Info%20Structure%20%28by%20ref%29) (EventInstigator :type Controller%20Object%20Reference))
  (bind (_hit _type) (Utilities|Struct|BreakMordhauDamageInfo DamageInfo))
  (if (CallFunction|IsCharacterType "NewEnumerator7")
    (Utilities|FlowControl|Sequence
      (:then_0
        (if (Variables|Default|GetIsImmortal)
          (return 0.0)))
      (:then_1
        (if (Utilities|Enum|Equal(Enum) _type "Fire")
          (LocalVariables|SetDamageMulti 0.25)))
      (:then_2
        (if (Utilities|Enum|Equal(Enum) _type "Ranged")
          (LocalVariables|SetDamageMulti 0.25)))
      (:then_3
        (bind _returnvalue (|CallParentFunction DamageAmount DamageInfo EventInstigator :!label _label))
        (Utilities|FlowControl|Sequence
          (:then_0
            (bind _asbp_supremacy_character (Utilities|Casting|CastToBP_SupremacyCharacter (Pawn|GetControlledPawn EventInstigator)))
            (bind _outdamage (CallFunction|ModifyOutgoingDamage _asbp_supremacy_character self _type _hit EventInstigator (LocalVariables|GetDamageMulti)))
            (LocalVariables|SetDamageMulti _outdamage))
          (:then_1
            (return (* (LocalVariables|GetDamageMulti) _returnvalue))))))
    (else
      (goto _label))))

(fn BeginHookshot
  (bind _asbp_supremacy_ability_motion (Utilities|Casting|CastToBP_SupremacyAbilityMotion (Class|AdvancedCharacter|GetMotion)))
  (Variables|/Script/Mordhau.MordhauMotion|SetEndTime _asbp_supremacy_ability_motion (+ (Variables|/Script/Mordhau.MordhauMotion|GetStartTime _asbp_supremacy_ability_motion) 1.0))
  (Variables|/PvEconquest/BP_SupremacyAbilityMotion.BP_SupremacyAbilityMotion_C|SetStage2Time _asbp_supremacy_ability_motion 0.5)
  (Class|AdvancedCharacter|PlayAnim (select (Variables|Default|GetbIsFirstPerson) "/Game/Mordhau/Animations/Montages/MTG_Horde_1P_Volley_V2.MTG_Horde_1P_Volley_V2" "/Game/Mordhau/Animations/Montages/MTG_Horde_Volley_V2.MTG_Horde_Volley_V2") 1.0 true))

(fn FindVolleyTarget
  (params (AimLocation :type Vector) (AimRotation :type Rotator))
  (bind (_outhit _returnvalue) (Collision|LineTraceForObjects AimLocation (+ AimLocation (* (Math|Vector|GetForwardVector AimRotation) 1e+04)) (Utilities|Array|MakeArray "ObjectTypeQuery1") true 0 "None"))
  (if _returnvalue
    (return true (.Location (Collision|BreakHitResult _outhit)))
    (else
      (return false "0, 0, 0"))))

(fn SpecialCooldown
  (params (Duration :type Float%20%28single-precision%29))
  (Networking|SwitchHasAuthority
    (:Authority
      (bind _asbp_supremacy_player_controller (Utilities|Casting|CastToBP_SupremacyPlayerController (Pawn|GetController)))
      (Variables|/PvEconquest/BP_SupremacyPlayerController.BP_SupremacyPlayerController_C|SetNextSpecialTime _asbp_supremacy_player_controller (+ Duration (Utilities|Time|GetTimeSeconds))))))

(fn Stage2Hookshot
  (Utilities|Casting|CastToBP_SupremacyAbilityMotion (Class|AdvancedCharacter|GetMotion))
  (Utilities|FlowControl|Sequence
    (:then_0
      (if (Pawn|IsLocallyControlled)
        (Audio|SpawnSound2D "/Game/Mordhau/Audio/Cues/Horde/Abilities/Soundcues/SC_ABL_VolleySting.SC_ABL_VolleySting" 1.0 1.0 0.0 0)
        (bind (_success _location) (CallFunction|FindVolleyTarget (Variables|Default|GetCameraLocation1P) (Variables|Default|GetCameraRotation1P)))
        (if _success
          (CallFunction|RequestVolley _location)
          (else
            (bind _asmordhau_player_controller (Utilities|Casting|CastToMordhauPlayerController (Pawn|GetController)))
            (Class|MordhauPlayerController|OnActionFailed _asmordhau_player_controller (Utilities|Name|MakeLiteralName "VolleyTarget"))))))))

(fn DoSpecialAbility
  (bind _special (Variables|Default|GetSpecial))
  (if (>= _special 1)
    (Utilities|Casting|CastToBP_AbilityMotion (Class|AdvancedCharacter|GetMotion)
      (:then
        _)
      (:CastFailed
        (Class|MordhauCharacter|AssignNetMotionSimple (Utilities|Enum|LiteralenumEMotionType "Ability") (Math|Conversions|ToByte(Integer) _special))
        (return true))))
  (return false))

(fn RememberStartAbilityTime
  (params (Duration :type Float%20%28single-precision%29))
  (Variables|Default|SetLastAbilityStartTime (Utilities|Time|GetTimeSeconds))
  (bind _output_get (Variables|Default|SetLastAbilityDuration Duration))
  (return _output_get))

(fn BeginShockwave
  (bind _asbp_supremacy_ability_motion (Utilities|Casting|CastToBP_SupremacyAbilityMotion (Class|AdvancedCharacter|GetMotion)))
  (Variables|/Script/Mordhau.MordhauMotion|SetEndTime _asbp_supremacy_ability_motion (+ (Variables|/Script/Mordhau.MordhauMotion|GetStartTime _asbp_supremacy_ability_motion) 1.0))
  (Variables|/PvEconquest/BP_SupremacyAbilityMotion.BP_SupremacyAbilityMotion_C|SetStage2Time _asbp_supremacy_ability_motion 0.5)
  (Class|AdvancedCharacter|PlayAnim (select (Variables|Default|GetbIsFirstPerson) "/Game/Mordhau/Animations/RawClips/Abilities/MTG_Shockwave_1P_V2.MTG_Shockwave_1P_V2" "/Game/Mordhau/Animations/RawClips/Abilities/MTG_Shockwave_V2.MTG_Shockwave_V2") 1.0 true))

(fn Stage2Shockwave
  (bind _self self)
  (Variables|Default|SetRagdollForceMultIfDmgAgent 17.0)
  (Variables|Default|SetbForceRagdollIfDmgAgent true)
  (Class|MordhauCharacter|PlayAttackYell)
  (Utilities|Casting|CastToBP_SupremacyAbilityMotion (Class|AdvancedCharacter|GetMotion))
  (Networking|SwitchHasAuthority
    (:Authority
      (CallFunction|SpecialCooldown 75.0)
      (Class|MordhauUtilityLibrary|MordhauApplyRadialDamagewithFalloff 5e+01 5e+01 0.0 0.0 (Transformation|GetActorLocation) 2.6e+02 2.6e+02 0.0 (Utilities|Array|MakeArray _self) 2.5e+03 0.0 5e+01 _self (Pawn|GetController) "ECC_Visibility" true "Generic"))))

(fn BeginImmortality
  (bind _asbp_supremacy_ability_motion (Utilities|Casting|CastToBP_SupremacyAbilityMotion (Class|AdvancedCharacter|GetMotion)))
  (Variables|/Script/Mordhau.MordhauMotion|SetEndTime _asbp_supremacy_ability_motion (+ (Variables|/Script/Mordhau.MordhauMotion|GetStartTime _asbp_supremacy_ability_motion) 1.0))
  (Variables|/PvEconquest/BP_SupremacyAbilityMotion.BP_SupremacyAbilityMotion_C|SetStage2Time _asbp_supremacy_ability_motion 0.25)
  (Class|AdvancedCharacter|PlayAnim (select (Variables|Default|GetbIsFirstPerson) "/Game/Mordhau/Animations/RawClips/Abilities/MTG_Immortality_1P_V2.MTG_Immortality_1P_V2" "/Game/Mordhau/Animations/RawClips/Abilities/MTG_Immortality_V2.MTG_Immortality_V2") 1.0 true))

(fn Stage2Immortality
  (Utilities|Casting|CastToBP_SupremacyAbilityMotion (Class|AdvancedCharacter|GetMotion))
  (CallFunction|RememberStartAbilityTime 5.0)
  (Utilities|FlowControl|Sequence
    (:then_0
      (if (Class|AdvancedCharacter|IsLocallyControlledIncludingVehicle)
        (bind _asmordhau_camera_manager (Utilities|Casting|CastToMordhauCameraManager (Game|GetPlayerCameraManager 0)))
        (Variables|/Script/Mordhau.MordhauCameraManager|SetHitFlashIgnoreUntilTime _asmordhau_camera_manager (+ (Variables|Default|GetLastAbilityStartTime) (Variables|Default|GetLastAbilityDuration)))))
    (:then_1
      (Networking|SwitchHasAuthority
        (:Authority
          (CallFunction|SpecialCooldown 8e+01)
          (CallFunction|TriggerImmortality))))))

(fn DebugCharacter
  (params (Message :type String))
  (bind _asbp_mordhau_player_controller (Utilities|Casting|CastToBP_MordhauPlayerController (Game|GetPlayerController 0)))
  (Default|RequestChatMessage _asbp_mordhau_player_controller Message false))

(fn IsCharacterType
  (params (Type :type ENUM_ConquestClasses%20Enum :default "NewEnumerator0"))
  (if (== (Variables|Default|GetCharacterType) Type)
    (return true)
    (else
      (return false))))

(fn ModifyOutgoingDamage
  (params (Receiver :type Actor%20Object%20Reference) (DamageType :type EMordhauDamageType%20Enum :default "Generic") (HitInfo :type Hit%20Result%20Structure%20%28by%20ref%29) (Agent :type Actor%20Object%20Reference) (InDamage :type Float%20%28single-precision%29))
  (Utilities|FlowControl|Sequence
    (:then_0
      (if (not (Utilities|Enum|Equal(Enum) DamageType "Melee"))
        (if (Utilities|Enum|Equal(Enum) DamageType "Ranged")
          (if (CallFunction|IsCharacterType "NewEnumerator2")
            (if (Math|Random|RandomBoolwithWeight 0.25)
              (LocalVariables|SetMultiplier (+ (LocalVariables|GetMultiplier) 0.5)))))))
    (:then_1
      (if (CallFunction|IsCharacterType "NewEnumerator3")
        (if (> (Class|KismetMathLibrary|DegAcos (Math|Vector|DotProduct (Transformation|GetActorForwardVector Receiver) (Math|Vector|Normalize (Math|Conversions|ToVector(Vector2D) (Math|Conversions|ToVector2D(Vector) (- (Transformation|GetActorLocation) (Transformation|GetActorLocation Receiver))))))) 9e+01)
          (LocalVariables|SetMultiplier (+ (LocalVariables|GetMultiplier) 0.25)))))
    (:then_2
      (if (CallFunction|IsCharacterType "NewEnumerator6")
        (Utilities|Casting|CastToBP_SupremacyEnemyCharacter Receiver)
        (LocalVariables|SetMultiplier (+ (LocalVariables|GetMultiplier) 0.25))))
    (:then_3
      (return (+ (LocalVariables|GetMultiplier) InDamage)))))

(fn AssignPerks
  (params (Perk :type Byte))
  (bind _returnvalue (Class|MordhauCharacter|GetCustomizationReplicationActor))
  (Utilities|IsValid _returnvalue
    (:Is%20Valid
      (if (Ability|HasAuthority _returnvalue)
        (if (not (Class|MordhauCharacter|HasPerk Perk))
          (bind _returnvalue_2 (Game|ConstructObjectfromClass "/Script/Mordhau.CharacterProfileBPWrapper" self))
          (bind _output_get (Variables|/Script/Mordhau.CharacterProfileBPWrapper|SetProfile _returnvalue_2 (Variables|/Script/Mordhau.CustomizationReplicationActor|GetLastAssignedProfile _returnvalue)))
          (Class|CharacterProfileBPWrapper|TogglePerk _returnvalue_2 Perk)
          (Class|CustomizationReplicationActor|AssignDatafromProfile _returnvalue _output_get))))))

(fn GiveFists
  (bind _equipment (Variables|Default|GetEquipment))
  (bind _returnvalue (Utilities|Array|Length _equipment))
  (bind _returnvalue_2 (- _returnvalue 1))
  (bind _output (Utilities|Array|Get(acopy) _equipment _returnvalue_2))
  (LocalVariables|SetDesiredFists "/Game/Mordhau/Blueprints/Equipment/Weapons/BP_PugilistFistsWeapon.BP_PugilistFistsWeapon_C")
  (Utilities|IsValid _output
    (:Is%20Valid
      (if (not (== (Utilities|GetClass _output) (LocalVariables|GetDesiredFists)))
        (bind _returnvalue_3 (Class|MordhauCharacter|DropEquipment _output true))
        (Actor|DestroyActor _returnvalue_3)
        (bind _returnvalue_4 (Game|SpawnActorfromClass (LocalVariables|GetDesiredFists) (Math|Transform|MakeTransform "0, 0, 0") "AlwaysSpawn" 0 0 :!label _label))
        (Class|MordhauCharacter|PickUptoSlot _returnvalue_4 (Math|Conversions|ToByte(Integer) (- (Utilities|Array|Length (Variables|Default|GetEquipment)) 1)))))
    (:Is%20Not%20Valid
      (goto _label))))

(fn OnRepStunnedbySkillCounter
  (Audio|SpawnSoundAttached "/Game/Mordhau/Audio/Cues/Horde/SC_Stunned.SC_Stunned" (Variables|Default|GetCapsuleComponent) "None" "0, 0, 0" "0, 0, 0" "SnapToTarget" false 1.0 1.0 0.0 0 0))

(fn DebugSupremacy
  (params (NewParam :type Text))
  (bind _asbp_mordhau_player_controller (Utilities|Casting|CastToBP_MordhauPlayerController (Game|GetPlayerController 0)))
  (Default|RequestChatMessage _asbp_mordhau_player_controller (Utilities|String|ToString(Text) NewParam) false))