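; Player state for the Supremacy mode that holds a replicated character type and coin count per player.
; On CopyProperties it casts the new player state and calls CopyFromOtherState, so both values carry over when the engine replaces the player state, such as during seamless travel.
; The RepNotify handlers for both variables are empty.
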(event EventBeginPlay
  (|CallParentFunction) ; This node is disabled and will not be called.\nDrag off pins to build functionality.
)

(event EventCopyProperties
  (params (NewPlayerState :type Player%20State%20Object%20Reference))
  (|CallParentFunction NewPlayerState)
  (bind _asbp_supremacy_player_state (Utilities|Casting|CastToBP_SupremacyPlayerState NewPlayerState))
  (CallFunction|CopyfromOtherState _asbp_supremacy_player_state self))

(fn ConstructionScript
  (|CallParentFunction))

(fn CopyfromOtherState
  (params (PlayerState :type BP%20Supremacy%20Player%20State%20Object%20Reference))
  (Variables|Default|SetCharacterType (Variables|BP_SupremacyPlayerState_C|GetCharacterType PlayerState))
  (Variables|Default|SetCoins (Variables|BP_SupremacyPlayerState_C|GetCoins PlayerState)))

(fn OnRepCoins)

(fn OnRepCharacterType)