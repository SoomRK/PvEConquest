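; Player controller for the Supremacy mode in Mordhau, handling class changes, hero specials and player feedback.
; Server requests spend PlayerState coins from class costs, then replicated CharacterType updates the special and triggers the spawn screen or respawn.
; It registers an Ability key at runtime, gates specials on server-time cooldown and routes score events to the HUD.
; Helpers grant customized equipment and roll recursion-guarded scattershot projectiles, with RepNotifies driving HUD and sound.
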(event Custom|ServerRequestChangeCharacter
  (params (CharacterType :type Byte))
  (bind _returnvalue (CallFunction|SpendCoins (.Cost (Utilities|Struct|BreakSTRUCT_ConquestClass_2 (.Value (Utilities|Map|Find (Variables|Default|GetClassMap) (Utilities|Enum|ByteToEnumENUM_ConquestClasses CharacterType)))))))
  (if _returnvalue
    (CallFunction|ChangeCharacter CharacterType)))

(event EventBeginPlay
  (|CallParentFunction)
  (Development|ExecuteConsoleCommand "m.NoTeamColorsOnGear 0" self)
  (Utilities|IsValid (Class|MordhauUtilityLibrary|GetMordhauInput) :!label _label
    (:Is%20Valid
      (CallFunction|AddMordhauInput (Utilities|Struct|MakeInputActionKeyMapping "Ability" false false false false "Six"))
      (bind _array_element (Utilities|Array|ForEachLoopwithBreak (Variables|/Script/Mordhau.MordhauInput|GetActionMappings (Class|MordhauUtilityLibrary|GetMordhauInput)) :!label _label_2)
        (:LoopBody
          (if (Utilities|Name|Equal(Name) (.ActionName (Utilities|Struct|BreakInputActionKeyMapping _array_element)) "Show Profile Select")
            (if (== (.Key (Utilities|Struct|BreakInputActionKeyMapping _array_element)) "None")
              (Utilities|Struct|SetmembersinInputActionKeyMapping _array_element "B")
              (goto _label_2 Break)
              (else
                (goto _label_2 Break)))))))
    (:Is%20Not%20Valid
      (Utilities|FlowControl|Delay 2.0)
      (goto _label))))

(event EventTick
  (params (DeltaSeconds :type Float%20%28single-precision%29))
  (|CallParentFunction DeltaSeconds) ; This node is disabled and will not be called.\nDrag off pins to build functionality.
)

(event EventOnMordhauCharacterSpawned
  (params (SpawnedCharacter :type Mordhau%20Character%20Object%20Reference)))

(event EventPossess
  (params (PossessedPawn :type Pawn%20Object%20Reference))
  (|CallParentFunction PossessedPawn)
  (bind _asbp_supremacy_character (Utilities|Casting|CastToBP_SupremacyCharacter PossessedPawn))
  (Variables|/PvEconquest/BP_SupremacyCharacter.BP_SupremacyCharacter_C|SetCharacterType _asbp_supremacy_character (Variables|Default|GetCharacterType)))

(event EventOnAfterPossess
  (params (aPawn :type Pawn%20Object%20Reference))
  (|CallParentFunction aPawn))

(event EventClientReceiveScoreBP
  (params (Reason :type EScoreFeedReason%20Enum :default "Kill") (ReasonParam :type Byte :default 0) (ScoreAmount :type Float%20%28single-precision%29) (AssociatedPlayer :type Mordhau%20Player%20State%20Object%20Reference))
  (bind _returnvalue (PlayerState|GetPlayerName AssociatedPlayer))
  (bind _returnvalue_2 (Math|Conversions|ToInteger(Byte) ReasonParam))
  (bind _hud (Variables|Default|GetHUD))
  (bind _scorefeed (Variables|/Game/Mordhau/Blueprints/BP_MordhauHUD.BP_MordhauHUD_C|GetScoreFeed _hud))
  (bind _crosshair (Variables|/Game/Mordhau/Blueprints/BP_MordhauHUD.BP_MordhauHUD_C|GetCrosshair _hud))
  (switch Utilities|FlowControl|Switch|SwitchonEScoreFeedReason Reason
    (:Kill
      (Utilities|IsValid AssociatedPlayer
        (:Is%20Valid
          (Default|AddKill _scorefeed ScoreAmount _returnvalue)
          (Default|ShowHitMarker _crosshair _returnvalue_2))))
    (:TeamKill
      (Utilities|IsValid AssociatedPlayer
        (:Is%20Valid
          (Default|AddTeamKill _scorefeed ScoreAmount _returnvalue))))
    (:Assist
      (Default|AddAssist _scorefeed ScoreAmount)
      (Audio|SpawnSound2D "/Game/Mordhau/Audio/Cues/UI/SC_ScoreGeneric.SC_ScoreGeneric" 1.0 1.0 0.0 0 :!label _label))
    (:Suicide
      (Default|AddSuicide _scorefeed ScoreAmount))
    (:PlayerDamage
      (Default|AddDamage _scorefeed ScoreAmount _returnvalue_2)
      (Default|ShowHitMarker _crosshair _returnvalue_2 :!label _label_2))
    (:PlayerTeamDamage
      (Default|AddTeamDamage _scorefeed ScoreAmount))
    (:OtherDamage
      (Default|AddStructureDamage _scorefeed ScoreAmount))
    (:Capturing
      (Default|AddCapturing _scorefeed ScoreAmount)
      (goto _label))
    (:Captured
      (Default|AddCaptured _scorefeed ScoreAmount))
    (:Neutralizing
      (Default|AddNeutralizing _scorefeed ScoreAmount)
      (goto _label))
    (:Neutralized
      (Default|AddNeutralized _scorefeed ScoreAmount))
    (:Objective
      (Default|AddObjective _scorefeed ScoreAmount)
      (goto _label))
    (:Heal
      (Default|AddHeal _scorefeed ScoreAmount)
      (goto _label))
    (:WaveCleared
      (Default|AddWaveCleared _scorefeed ScoreAmount)
      (goto _label))
    (:Repair
      (Default|AddRepair _scorefeed ScoreAmount)
      (goto _label_2))
    (:VehicleDamage
      (Default|AddVehicleDamage _scorefeed ScoreAmount)
      (goto _label_2))
    (:VehicleTeamDamage
      (Default|AddVehicleTeamDamage _scorefeed ScoreAmount))
    (:Spawn
      (Default|AddSpawn _scorefeed ScoreAmount)
      (goto _label))))

(event Input|ActionEvents|InputActionAbility
  (params (Key :type Key%20Structure :default "None"))
  (bind _returnvalue (Game|GetGameState))
  (:Pressed
    (bind _asbp_supremacy_character (Utilities|Casting|CastToBP_SupremacyCharacter (Pawn|GetControlledPawn)))
    (if (and (>= (Variables|/PvEconquest/BP_SupremacyCharacter.BP_SupremacyCharacter_C|GetSpecial _asbp_supremacy_character) 1) (not (Class|AdvancedCharacter|GetIsDead _asbp_supremacy_character)))
      (Utilities|IsValid _returnvalue
        (:Is%20Valid
          (if (>= (GameState|GetServerWorldTimeSeconds _returnvalue) (Variables|Default|GetNextSpecialTime))
            (bind _success (Default|DoSpecialAbility _asbp_supremacy_character))
            (if (not _success)
              (Class|MordhauPlayerController|OnActionFailed (Utilities|Name|MakeLiteralName "None") :!label _label))
            (else
              (goto _label))))))))

(event Input|ActionEvents|InputActionShowProfileSelect
  (params (Key :type Key%20Structure :default "None"))
  (:Pressed
    (CallFunction|ShowMenu)))

(fn ConstructionScript
  (|CallParentFunction))

(fn AddMordhauInput
  (params (Input%20Action :type Input%20Action%20Key%20Mapping%20Structure))
  (bind _returnvalue (Class|MordhauUtilityLibrary|GetMordhauInput))
  (bind _actionmappings (Variables|/Script/Mordhau.MordhauInput|GetActionMappings _returnvalue))
  ;[1 1 1] NOTE: You need to make Input action inside Unreal Project settings to be able to get the event for this input action
  (bind _array_element (Utilities|Array|ForEachLoopwithBreak _actionmappings :!label _label)
    (:LoopBody
      (if (Utilities|Name|Equal(Name) (.ActionName (Utilities|Struct|BreakInputActionKeyMapping _array_element)) (.ActionName (Utilities|Struct|BreakInputActionKeyMapping Input%20Action)))
        (LocalVariables|SetAlreadyExists true)
        (goto _label Break)))
    (:Completed
      (if (LocalVariables|GetAlreadyExists)
        (return false)
        (else
          (Utilities|Array|Add _actionmappings Input%20Action)
          (Class|MordhauInput|SaveSettings _returnvalue)
          (Class|MordhauInput|ApplySettings _returnvalue)
          (return true))))))

(fn OnRepNextSpecialTime
  (bind _asbp_supremacy_game_state (Utilities|Casting|CastToBP_SupremacyGameState (Game|GetGameState)))
  (Variables|Default|SetSpecialTriggeredTime (GameState|GetServerWorldTimeSeconds _asbp_supremacy_game_state))
  (bind _asbp_supremacy_hud (Utilities|Casting|CastToBP_SupremacyHUD (Class|MordhauUtilityLibrary|GetMordhauHUD)))
  (Default|UltimateUsed (Variables|/PvEconquest/Widgets/BP_SupremacyHudWidget2.BP_SupremacyHudWidget2_C|GetBP_UltimateDisplay_Supremacy (Variables|/PvEconquest/BP_SupremacyHUD.BP_SupremacyHUD_C|GetSupremacyHudWidget _asbp_supremacy_hud))))

(fn OnRepPurchaseTrigger
  (Networking|CanExecuteCosmeticEvents
    (:True
      (Audio|PlaySound2D "/Game/Mordhau/Audio/Cues/UI/SC_HordePurchaseItem.SC_HordePurchaseItem" 1.0 1.0 0.0 0 0))))

(fn AssignFireArrowValues
  (params (Arrow :type Actor%20Object%20Reference))
  (bind _asbp_arrow_projectile (Utilities|Casting|CastToBP_ArrowProjectile Arrow)))

(fn TryScatterShot
  (params (SourceProjectile :type Mordhau%20Projectile%20Object%20Reference))
  (bind _returnvalue (Utilities|GetClass SourceProjectile))
  (bind _returnvalue_2 (Transformation|GetActorTransform SourceProjectile))
  (bind (_location _rotation _scale) (Math|Transform|BreakTransform _returnvalue_2))
  (bind (_roll _pitch _yaw) (Math|Rotator|BreakRotator _rotation))
  (bind (_roll_2 _pitch_2 _yaw_2) (Math|Rotator|BreakRotator _rotation))
  (if (Math|Random|RandomBoolwithWeight 0.25)
    (Networking|SwitchHasAuthority
      (:Authority
        (if (not (Variables|Default|GetAvoidScattershotRecursion))
          (Variables|Default|SetAvoidScattershotRecursion true)
          (Utilities|FlowControl|Sequence
            (:then_0
              (bind _returnvalue_3 (Class|MordhauPlayerController|GetLastControlledCharacter))
              (Utilities|IsValid _returnvalue_3
                (:Is%20Valid
                  (Utilities|FlowControl|Sequence
                    (:then_0
                      (bind _returnvalue_4 (Game|SpawnActorfromClass _returnvalue (Math|Transform|MakeTransform (Math|Transform|TransformLocation _returnvalue_2 "50.000000,10.000000, 0") (Math|Rotator|MakeRotator _roll _pitch (+ _yaw 2.5)) _scale) "Undefined" 0 0))
                      (Variables|/Script/Mordhau.MordhauProjectile|SetbUsesLocalProjectileBlending _returnvalue_4 false)
                      (CallFunction|AssignFireArrowValues _returnvalue_4)
                      (Class|MordhauProjectile|InitializeProjectile _returnvalue_4 self false _returnvalue_3)
                      (Class|MordhauProjectile|Fire _returnvalue_4)
                      (Variables|Default|SetScattershotCounter (+ (Variables|Default|GetScattershotCounter) 1)))
                    (:then_1
                      (bind _returnvalue_5 (Game|SpawnActorfromClass _returnvalue (Math|Transform|MakeTransform (Math|Transform|TransformLocation _returnvalue_2 "50.000000,-10.000000, 0") (Math|Rotator|MakeRotator _roll_2 _pitch_2 (+ _yaw_2 -2.5)) _scale) "Undefined" 0 0))
                      (Variables|/Script/Mordhau.MordhauProjectile|SetbUsesLocalProjectileBlending _returnvalue_5 false)
                      (CallFunction|AssignFireArrowValues _returnvalue_5)
                      (Class|MordhauProjectile|InitializeProjectile _returnvalue_5 self false _returnvalue_3)
                      (Class|MordhauProjectile|Fire _returnvalue_5))))))
            (:then_1
              (Variables|Default|SetAvoidScattershotRecursion false))))))))

(fn OnRepScattershotCounter
  (bind _asbp_supremacy_hud (Utilities|Casting|CastToBP_SupremacyHUD (Variables|Default|GetHUD)))
  (Default|AddSkill (Variables|/PvEconquest/Widgets/BP_SupremacyHudWidget2.BP_SupremacyHudWidget2_C|GetBP_PassiveSkillFeed (Variables|/PvEconquest/BP_SupremacyHUD.BP_SupremacyHUD_C|GetSupremacyHudWidget _asbp_supremacy_hud)) "Scattershot!" "/Game/Mordhau/UI/UIAssets/Textures/SkillIcons/IC_Skill_Scattershot.IC_Skill_Scattershot"))

(fn ShowMenu
  (bind _asbp_supremacy_hud (Utilities|Casting|CastToBP_SupremacyHUD (Class|MordhauUtilityLibrary|GetMordhauHUD)))
  (Default|ShowCustomProfileSelect _asbp_supremacy_hud))

(fn SpendCoins
  (params (Coins :type Integer))
  (if (== Coins 0)
    (return true)
    (else
      (bind _asbp_supremacy_player_state (Utilities|Casting|CastToBP_SupremacyPlayerState (Variables|Default|GetPlayerState)))
      (if (>= (Variables|/PvEconquest/BP_SupremacyPlayerState.BP_SupremacyPlayerState_C|GetCoins _asbp_supremacy_player_state) Coins)
        (Variables|/PvEconquest/BP_SupremacyPlayerState.BP_SupremacyPlayerState_C|SetCoins _asbp_supremacy_player_state (- (Variables|/PvEconquest/BP_SupremacyPlayerState.BP_SupremacyPlayerState_C|GetCoins _asbp_supremacy_player_state) Coins))
        (return true)
        (else
          (return false))))))

(fn GiveItem
  (params (ClassToBuy :type Mordhau%20Actor%20Class%20Reference))
  (bind _characterprofile (Variables|Default|GetCharacterProfile))
  (bind _appearancecustomization (Utilities|Struct|BreakCharacterProfile _characterprofile))
  (bind (_emblem _emblemcolors) (Utilities|Struct|BreakAppearanceCustomization _appearancecustomization))
  (bind _asbp_mordhau_character (Utilities|Casting|CastToBP_MordhauCharacter (Pawn|GetControlledPawn)))
  (if (Utilities|IsValidClass ClassToBuy)
    (bind _returnvalue (Game|SpawnActorfromClass ClassToBuy (Transformation|GetActorTransform _asbp_mordhau_character) "Undefined" 0 0))
    (bind _asmordhau_equipment (Utilities|Casting|CastToMordhauEquipment _returnvalue)
      (:then
        (bind _returnvalue_2 (Class|MordhauEquipment|GetRandomCustomization _asmordhau_equipment true))
        (LocalVariables|SetCustomization _returnvalue_2)
        (Utilities|FlowControl|Sequence
          (:then_0
            (LocalVariables|SetEmblem _emblem)
            (LocalVariables|SetEmblemColor1 (Utilities|Array|Get(acopy) _emblemcolors))
            (LocalVariables|SetEmblemColor2 (Utilities|Array|Get(acopy) _emblemcolors 1))
            (bind (_outcustomization _returnvalue_3) (Class|MordhauPlayerController|GetDefaultEquipmentCustomizationfor (Utilities|GetClass _asmordhau_equipment)))
            (if _returnvalue_3
              (LocalVariables|SetCustomization _outcustomization)))
          (:then_1
            (Class|MordhauEquipment|AssignCustomization _asmordhau_equipment (LocalVariables|GetCustomization) (Math|Conversions|ToByte(Integer) (LocalVariables|GetEmblem)) (LocalVariables|GetEmblemColor1) (LocalVariables|GetEmblemColor2))
            (bind _returnvalue_4 (Class|MordhauCharacter|PickUp _asbp_mordhau_character _asmordhau_equipment -1))
            (if _returnvalue_4
              (Class|MordhauCharacter|SwitchEquipment _asbp_mordhau_character _asmordhau_equipment)
              (else
                (Variables|/Script/Mordhau.MordhauEquipment|SetbCanRagdoll _asmordhau_equipment true)
                (Class|MordhauEquipment|UpdateEquipmentState _asmordhau_equipment))))))
      (:CastFailed
        (bind _asbp_wearable_pickup (Utilities|Casting|CastToBP_WearablePickup _returnvalue))
        (Default|Equip _asbp_wearable_pickup _asbp_mordhau_character)))))

(fn ChangeCharacter
  (params (Character :type Byte))
  (Utilities|FlowControl|Sequence
    (:then_0
      (if (<= Character 2)
        (Networking|SwitchHasAuthority
          (:Authority
            (Variables|Default|SetLast%20Character%20Type Character)))))
    (:then_1
      (bind _asbp_supremacy_player_state (Utilities|Casting|CastToBP_SupremacyPlayerState (Variables|Default|GetPlayerState)))
      (Networking|SwitchHasAuthority
        (:Authority
          (Variables|/PvEconquest/BP_SupremacyPlayerState.BP_SupremacyPlayerState_C|SetCharacterType _asbp_supremacy_player_state Character)
          (Variables|Default|SetCharacterType Character))))))

(fn OnRepCharacterType
  (bind _returnvalue (Class|MordhauPlayerController|GetControlledMordhauCharacter true))
  (CallFunction|SetSpecial)
  (Utilities|IsValid _returnvalue
    (:Is%20Valid
      (if (Class|AdvancedCharacter|GetIsDead _returnvalue)
        (bind _asbp_supremacy_hud (Utilities|Casting|CastToBP_SupremacyHUD (HUD|GetHUD) :!label _label))
        (Default|ShowSpawnScreen _asbp_supremacy_hud)
        (else
          (bind _returnvalue_2 (Class|PlayerController|CanRestartPlayer))
          (if _returnvalue_2
            (bind _asbp_mordhau_game_mode (Utilities|Casting|CastToBP_MordhauGameMode (Game|GetGameMode)))
            (Default|UnpossessandDestroyPawn _asbp_mordhau_game_mode self true)))))
    (:Is%20Not%20Valid
      (goto _label))))

(fn OnRepLastCharacterType)

(fn SetSpecial
  (switch Utilities|FlowControl|Switch|SwitchonENUM_ConquestClasses (Utilities|Enum|ByteToEnumENUM_ConquestClasses (Variables|Default|GetCharacterType))
    (:NewEnumerator0
      (Variables|Default|SetCurrentSpecial "NewEnumerator0" :!label _label))
    (:NewEnumerator1
      (goto _label))
    (:NewEnumerator2
      (goto _label))
    (:NewEnumerator3
      (goto _label))
    (:NewEnumerator4
      (goto _label))
    (:NewEnumerator5
      (goto _label))
    (:NewEnumerator6
      (Variables|Default|SetCurrentSpecial "NewEnumerator1")
      (bind _asbp_supremacy_hud (Utilities|Casting|CastToBP_SupremacyHUD (Class|MordhauUtilityLibrary|GetMordhauHUD) :!label _label_2))
      (Default|ChangeIcon (Variables|/PvEconquest/Widgets/BP_SupremacyHudWidget2.BP_SupremacyHudWidget2_C|GetBP_UltimateDisplay_Supremacy (Variables|/PvEconquest/BP_SupremacyHUD.BP_SupremacyHUD_C|GetSupremacyHudWidget _asbp_supremacy_hud)))
      (Networking|SwitchHasAuthority
        (:Authority
          (Variables|Default|SetNextSpecialTime (+ 75.0 (Utilities|Time|GetTimeSeconds))))))
    (:NewEnumerator7
      (Variables|Default|SetCurrentSpecial "NewEnumerator2")
      (goto _label_2))
    (:NewEnumerator8
      (Variables|Default|SetCurrentSpecial "NewEnumerator3")
      (goto _label_2))
    (:NewEnumerator9
      (goto _label))))