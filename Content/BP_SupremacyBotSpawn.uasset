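; BP_SupremacyBotSpawn is a team-specific bot spawn actor that reports how many bots its team is missing.
; GetAliveBots scans all BP_SupremacyEnemyCharacter actors, counts living ones on the same Team, and returns BotCount minus that count, along with the Team.
; The event graph has no active logic, and the file performs no spawning itself.
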(event EventBeginPlay
  (|CallParentFunction) ; This node is disabled and will not be called.\nDrag off pins to build functionality.
)

(event EventTick
  (params (DeltaSeconds :type Float%20%28single-precision%29))
  (|CallParentFunction DeltaSeconds) ; This node is disabled and will not be called.\nDrag off pins to build functionality.
)

(fn ConstructionScript
  (|CallParentFunction))

(fn GetAliveBots
  (bind _outactors (Actor|GetAllActorsOfClass "/PvEconquest/BP_SupremacyEnemyCharacter.BP_SupremacyEnemyCharacter_C"))
  (for _array_element _outactors
    (if (== (Variables|Default|GetTeam) (Variables|/Script/Mordhau.AdvancedCharacter|GetTeam _array_element))
      (if (not (Class|AdvancedCharacter|GetIsDead _array_element))
        (LocalVariables|SetBotsAlive (+ (LocalVariables|GetBotsAlive) 1)))))
  (return (- (Variables|Default|GetBotCount) (LocalVariables|GetBotsAlive)) (Variables|Default|GetTeam)))