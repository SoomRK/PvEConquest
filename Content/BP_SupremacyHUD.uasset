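; BP_SupremacyHUD is the Supremacy mode HUD, extending a parent HUD that appears to be the Frontline one.
; On game state replication it polls until FrontlineHUDWidget is valid, then adds the Supremacy HUD widget and a collapsed BP_SupremacyMenu.
; Main-menu and minimal/full HUD events toggle the Supremacy widget's visibility after calling the parent.
; ShowProfileSelect shows the Supremacy menu instead of calling its parent; spawn-screen rebinding code is unconnected.
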(event Custom|CustomEvent_0
  (CallFunction|ShowCustomProfileSelect))

(event EventBeginPlay
  (|CallParentFunction) ; This node is disabled and will not be called.\nDrag off pins to build functionality.
)

(event Collision|EventActorBeginOverlap
  (params (OtherActor :type Actor%20Object%20Reference)))

(event EventHideMainMenu
  (bind _supremacyhudwidget (Variables|Default|GetSupremacyHudWidget))
  (|CallParentFunction)
  (Utilities|IsValid _supremacyhudwidget
    (:Is%20Valid
      (Widget|SetVisibility _supremacyhudwidget "Visible"))))

(event EventOnGameStateReplicated
  (|CallParentFunction)
  (Utilities|IsValid (Variables|Default|GetFrontlineHUDWidget) :!label _label
    (:Is%20Valid
      (Utilities|FlowControl|Sequence
        (:then_0
          (bind _returnvalue (UserInterface|CreateWidget "/PvEconquest/Widgets/BP_SupremacyHudWidget2.BP_SupremacyHudWidget2_C" (Game|GetPlayerController 0)))
          (bind _output_get (Variables|Default|SetSupremacyHudWidget _returnvalue))
          (UserInterface|Viewport|AddtoViewport _output_get -5)
          (if (Variables|Default|GetIsHUDMinimal)
            (Widget|SetVisibility _output_get "Hidden")))
        (:then_1
          (CallFunction|MakeProfileSelect))))
    (:Is%20Not%20Valid
      (Utilities|FlowControl|Delay 0.5)
      (goto _label))))

(event EventTick
  (params (DeltaSeconds :type Float%20%28single-precision%29))
  (|CallParentFunction DeltaSeconds) ; This node is disabled and will not be called.\nDrag off pins to build functionality.
)

(event EventShowMainMenu
  (bind _supremacyhudwidget (Variables|Default|GetSupremacyHudWidget))
  (|CallParentFunction)
  (Utilities|IsValid _supremacyhudwidget
    (:Is%20Valid
      (Widget|SetVisibility _supremacyhudwidget "Hidden"))))

(event EventUseMinimalHUD
  (bind _supremacyhudwidget (Variables|Default|GetSupremacyHudWidget))
  (|CallParentFunction)
  (Utilities|IsValid _supremacyhudwidget
    (:Is%20Valid
      (Widget|SetVisibility _supremacyhudwidget "Hidden"))))

(event EventUseFullHUD
  (bind _supremacyhudwidget (Variables|Default|GetSupremacyHudWidget))
  (|CallParentFunction)
  (Utilities|IsValid _supremacyhudwidget
    (:Is%20Valid
      (Widget|SetVisibility _supremacyhudwidget "Visible"))))

(fn ConstructionScript
  (|CallParentFunction))

(fn MakeProfileSelect
  (bind _returnvalue (UserInterface|CreateWidget "/PvEconquest/Widgets/BP_SupremacyMenu.BP_SupremacyMenu_C" (Game|GetPlayerController 0)))
  (bind _output_get (Variables|Default|SetConquestMenu _returnvalue))
  (UserInterface|Viewport|AddtoViewport _output_get 7)
  (Widget|SetVisibility _output_get "Collapsed"))

(fn NewFunction0)

(fn ShowCustomProfileSelect
  (Default|Show (Variables|Default|GetConquestMenu)))

(fn ShowProfileSelect
  (CallFunction|ShowCustomProfileSelect))

(fn CreateSpawnScreen
  (|CallParentFunction))

(fn CreateTeamSelect
  (|CallParentFunction))

(fn ShowSpawnScreen
  (|CallParentFunction))