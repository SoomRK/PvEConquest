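; BP_CrushCharacter is a character Blueprint that currently adds no behavior of its own over its parent class.
; Its event graph holds only disabled default events, and its construction script just calls the parent.
; The ModifyDamage override returns the parent's result unchanged; a node scaling that result by 0.9 is left unused, so no damage reduction applies here.
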(event EventBeginPlay
  (|CallParentFunction) ; This node is disabled and will not be called.\nDrag off pins to build functionality.
)

(event Collision|EventActorBeginOverlap
  (params (OtherActor :type Actor%20Object%20Reference))
  (|CallParentFunction OtherActor) ; This node is disabled and will not be called.\nDrag off pins to build functionality.
)

(event EventTick
  (params (DeltaSeconds :type Float%20%28single-precision%29))
  (|CallParentFunction DeltaSeconds) ; This node is disabled and will not be called.\nDrag off pins to build functionality.
)

(fn ConstructionScript
  (|CallParentFunction))

(fn ModifyDamage
  (params (DamageAmount :type Float%20%28single-precision%29) (DamageInfo :type Mordhau%20Damage%20Info%20Structure%20%28by%20ref%29) (EventInstigator :type Controller%20Object%20Reference))
  (bind _returnvalue (|CallParentFunction DamageAmount DamageInfo EventInstigator))
  (return _returnvalue))