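; Motion that plays a Supremacy character's ability: Shockwave, Immortality or Hookshot, selected by MotionParam0 of the current net motion.
; On begin it resets the character's additive override type and calls that ability's Begin function on BP_SupremacyCharacter.
; Tick counts down Stage2Time, then makes a one-time call to the matching Stage2 function on the character.
; If the motion is interrupted, it destroys any valid Projectile.
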(event EventOnBegin
  (|CallParentFunction)
  (bind _asbp_supremacy_character (Utilities|Casting|CastToBP_SupremacyCharacter (Class|MordhauMotion|GetOwnerMordhauCharacter)))
  (Class|AdvancedCharacter|ResetAdditiveOverrideType _asbp_supremacy_character)
  (switch int (Math|Conversions|ToInteger(Byte) (.MotionParam0 (Utilities|Struct|BreakNetMotion (Class|MordhauCharacter|GetCurrentNetMotion _asbp_supremacy_character))))
    (:1
      (Default|BeginShockwave _asbp_supremacy_character))
    (:2
      (Default|BeginImmortality _asbp_supremacy_character))
    (:3
      (Default|BeginHookshot _asbp_supremacy_character))))

(event EventOnTick
  (params (DeltaTime :type Float%20%28single-precision%29))
  (|CallParentFunction DeltaTime)
  (if (== (Variables|Default|GetCurrentStage) 0)
    (bind _output_get (Variables|Default|SetStage2Time (- (Variables|Default|GetStage2Time) DeltaTime)))
    (if (<= _output_get 0.0)
      (Variables|Default|SetCurrentStage 1)
      (bind _asbp_supremacy_character (Utilities|Casting|CastToBP_SupremacyCharacter (Class|MordhauMotion|GetOwnerMordhauCharacter)))
      (switch int (Math|Conversions|ToInteger(Byte) (.MotionParam0 (Utilities|Struct|BreakNetMotion (Class|MordhauCharacter|GetCurrentNetMotion _asbp_supremacy_character))))
        (:1
          (Default|Stage2Shockwave _asbp_supremacy_character))
        (:2
          (Default|Stage2Immortality _asbp_supremacy_character))
        (:3
          (Default|Stage2Hookshot _asbp_supremacy_character))))))

(event EventOnLeave
  (params (Interrupted :type Boolean))
  (bind _projectile (Variables|Default|GetProjectile))
  (|CallParentFunction Interrupted)
  (if Interrupted
    (Utilities|IsValid _projectile
      (:Is%20Valid
        (Actor|DestroyActor _projectile)))))