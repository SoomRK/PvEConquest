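; Enemy character for Supremacy mode that knocks back nearby living players when possessed and kills itself if left without a controller.
; Incoming damage is scaled by the attacking player's modifiers, kicks bypass its parry, and melee deaths trigger the killer's team heal.
; Player skills drive timed cripple and enrage states, plus a chance-based stun with replicated sound.
; It damages blocking destroyables and pavise shields, massively so shortly after climbing or possession.
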(event Custom|Cripple
  (params (Duration :type Float%20%28single-precision%29))
  (bind _charactermovement (Variables|Character|GetCharacterMovement))
  (if (not (Class|AdvancedCharacter|GetIsDead))
    (if (not (Variables|Default|GetIsBoss))
      (Utilities|FlowControl|Sequence
        (:then_0
          (if (not (Variables|Default|GetIsCrippled))
            (Variables|Default|SetPreCrippleMaxWalkSpeed (Variables|/Script/Engine.CharacterMovementComponent|GetMaxWalkSpeed _charactermovement))
            (Variables|Default|SetIsCrippled true)
            (Variables|/Script/Engine.CharacterMovementComponent|SetMaxWalkSpeed _charactermovement (* (Variables|/Script/Engine.CharacterMovementComponent|GetMaxWalkSpeed _charactermovement) 0.5))))
        (:then_1
          (Utilities|FlowControl|RetriggerableDelay Duration)
          (if (not (Class|AdvancedCharacter|GetIsDead))
            (Variables|Default|SetIsCrippled false)
            (Variables|/Script/Engine.CharacterMovementComponent|SetMaxWalkSpeed _charactermovement (Variables|Default|GetPreCrippleMaxWalkSpeed))))))))

(event Custom|Enrage
  (params (Target :type Mordhau%20Character%20Object%20Reference) (Duration :type Float%20%28single-precision%29))
  (Variables|Default|SetRageTarget Target)
  (Utilities|FlowControl|RetriggerableDelay Duration)
  (Variables|Default|SetRageTarget 0))

(event EventBeginPlay
  (|CallParentFunction)
  (Utilities|FlowControl|Delay 5.0)
  (Utilities|IsValid (Class|AdvancedCharacter|GetControllerIncludingVehicle)
    (:Is%20Not%20Valid
      (Game|Damage|ApplyDamage 0 6969.0 0 0))))

(event EventOnDied
  (params (Angle :type Float%20%28single-precision%29) (Type :type EMordhauDamageType%20Enum :default "Generic") (SubType :type Byte :default 0) (Bone :type Name :default "None") (Point :type Vector :default "0, 0, 0") (Source :type Actor%20Object%20Reference) (Agent :type Actor%20Object%20Reference))
  (Variables|/Script/Mordhau.MordhauWidgetComponent|SetOverrideVisible (Variables|Default|GetMordhauWidget) 0)
  (|CallParentFunction Angle Type SubType Bone Point Source Agent))

(event EventMoveBlockedbySlow
  (params (Impact :type Hit%20Result%20Structure%20%28by%20ref%29))
  (CallFunction|HandleObstructionRemoval Impact))

(event EventMordhauDamage
  (params (Damage :type Float%20%28single-precision%29) (HitResult :type Hit%20Result%20Structure) (DamageType :type EMordhauDamageType%20Enum :default "Generic") (SubDamageType :type Byte :default 0) (Source :type Actor%20Object%20Reference) (Agent :type Actor%20Object%20Reference) (EventInstigator :type Controller%20Object%20Reference))
  (|CallParentFunction Damage HitResult DamageType SubDamageType Source Agent EventInstigator))

(event EventOnBlockedMelee
  (params (HitResult :type Hit%20Result%20Structure%20%28by%20ref%29) (Attacker :type Mordhau%20Character%20Object%20Reference))
  (|CallParentFunction HitResult Attacker)
  (if (Class|AdvancedCharacter|GetIsDead)
    (bind _asbp_supremacy_character (Utilities|Casting|CastToBP_SupremacyCharacter Attacker))
    (if (Default|IsCharacterType _asbp_supremacy_character "NewEnumerator6")
      (if (Math|Random|RandomBoolwithWeight 0.35)
        (Class|MordhauCharacter|AssignNetMotionSimple (Utilities|Enum|LiteralenumEMotionType "Stunned") 127)
        (Variables|Default|SetStunnedBySkillCounter (+ (Variables|Default|GetStunnedBySkillCounter) 1))))))

(event EventOnKilled
  (params (EventInstigator :type Controller%20Object%20Reference))
  (|CallParentFunction EventInstigator)
  (bind _returnvalue (Class|AdvancedCharacter|GetLastNetDamageType))
  (if (Utilities|Enum|Equal(Enum) _returnvalue "Melee")
    (bind _returnvalue_2 (Class|AdvancedCharacter|GetLastNetDamageSource))
    (bind _asbp_supremacy_character (Utilities|Casting|CastToBP_SupremacyCharacter _returnvalue_2))
    (Default|AwardHealthonKilltoTeammates _asbp_supremacy_character)))

(event EventPossessed
  (params (NewController :type Controller%20Object%20Reference))
  (|CallParentFunction NewController)
  (bind _outactors (Collision|SphereOverlapActors (Transformation|GetActorLocation) 1e+02 (Utilities|Array|MakeArray "ObjectTypeQuery3") "/PvEconquest/BP_SupremacyCharacter.BP_SupremacyCharacter_C"))
  (for _array_element _outactors
    (bind _asmordhau_character (Utilities|Casting|CastToMordhauCharacter _array_element))
    (if (not (Class|AdvancedCharacter|GetIsDead _asmordhau_character))
      (bind _returnvalue (Class|MordhauCharacter|IsinKnockback _asmordhau_character))
      (if (not _returnvalue)
        (Class|AdvancedCharacter|Knockback _asmordhau_character (* (Math|Vector|Normalize (- (Transformation|GetActorLocation _asmordhau_character) (Transformation|GetActorLocation))) 1e+03))))))

(fn ConstructionScript
  (|CallParentFunction))

(fn ModifyDamage
  (params (DamageAmount :type Float%20%28single-precision%29) (DamageInfo :type Mordhau%20Damage%20Info%20Structure%20%28by%20ref%29) (EventInstigator :type Controller%20Object%20Reference))
  (bind (_hit _type _subtype _damagesource _damageagent) (Utilities|Struct|BreakMordhauDamageInfo DamageInfo))
  (bind _returnvalue (|CallParentFunction DamageAmount DamageInfo EventInstigator))
  (Utilities|FlowControl|Sequence
    (:then_0
      (bind _asbp_supremacy_player_controller (Utilities|Casting|CastToBP_SupremacyPlayerController EventInstigator))
      (bind _asbp_supremacy_character (Utilities|Casting|CastToBP_SupremacyCharacter (Pawn|GetControlledPawn _asbp_supremacy_player_controller)))
      (bind _outdamage (Default|ModifyOutgoingDamage _asbp_supremacy_character self _type _hit _damageagent (LocalVariables|GetDamageMulti)))
      (LocalVariables|SetDamageMulti _outdamage))
    (:then_1
      (return (* (LocalVariables|GetDamageMulti) _returnvalue)))))

(fn ModifyParryResult
  (params (InResult :type Boolean) (HitResult :type Hit%20Result%20Structure%20%28by%20ref%29) (Attacker :type Mordhau%20Character%20Object%20Reference))
  (Utilities|Casting|CastToKickMotion (Variables|/Script/Mordhau.MotionSystemComponent|GetLastAttackMotion (Variables|/Script/Mordhau.AdvancedCharacter|GetMotionSystemComponent Attacker))
    (:then
      (return false))
    (:CastFailed
      (bind _returnvalue (|CallParentFunction InResult HitResult Attacker))
      (return _returnvalue))))

(fn GetEnragedTarget
  (bind _ragetarget (Variables|Default|GetRageTarget))
  (Utilities|IsValid _ragetarget
    (:Is%20Valid
      (if (Class|AdvancedCharacter|GetIsDead _ragetarget)
        _
        (else
          (return _ragetarget))))
    (:Is%20Not%20Valid
      _))
  (return 0))

(fn OnRepStunnedbySkillCounter
  (Audio|SpawnSoundAttached "/Game/Mordhau/Audio/Cues/Horde/SC_Stunned.SC_Stunned" (Variables|Default|GetCapsuleComponent) "None" "0, 0, 0" "0, 0, 0" "SnapToTarget" false 1.0 1.0 0.0 0 0))

(fn HandleObstructionRemoval
  (params (Impact :type Hit%20Result%20Structure))
  (bind _hitactor (Collision|BreakHitResult Impact))
  (LocalVariables|SetDamageToApply (Variables|Default|GetWoodDamageForPathClearing))
  (bind _output_get (LocalVariables|SetExtraDamageMode (or (> (+ (Variables|Default|GetLastClimbTime) 3.0) (Utilities|Time|GetTimeSeconds)) (> (+ (Variables|Default|GetLastPossessionTime) 1.0) (Utilities|Time|GetRealTimeSeconds)))))
  (Utilities|FlowControl|Sequence
    (:then_0
      (if _output_get
        (LocalVariables|SetDamageToApply 99999.0)))
    (:then_1
      (Utilities|Casting|CastToBP_DestroyableActor _hitactor
        (:then
          _)
        (:CastFailed
          (Utilities|Casting|CastToBP_PaviseShield _hitactor)))
      (Game|Damage|ApplyDamage _hitactor (LocalVariables|GetDamageToApply) (Pawn|GetController) self))))

(fn AttemptClimb
  (Variables|Default|SetLastClimbTime (Utilities|Time|GetTimeSeconds))
  (bind _succeeded (|CallParentFunction))
  (return _succeeded))