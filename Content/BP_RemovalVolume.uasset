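; BP_RemovalVolume is a box volume that removes level geometry overlapping it at runtime.
; One second after BeginPlay, it gathers the actors overlapping its Box and destroys any StaticMeshActor or LODActor, so HLOD proxy actors are removed along with meshes.
; Each matching actor is switched to replicated immediately before it is destroyed.
; The check runs once, with no Tick or overlap-event logic.
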(event EventBeginPlay
  (|CallParentFunction)
  (Utilities|FlowControl|Delay 1.0)
  (for _array_element (Collision|GetOverlappingActors (Variables|Default|GetBox) 0 :!class /Script/Engine.PrimitiveComponent)
    (bind _asstatic_mesh_actor (Utilities|Casting|CastToStaticMeshActor _array_element)
      (:then
        (Networking|SetReplicates _asstatic_mesh_actor true)
        (Actor|DestroyActor _asstatic_mesh_actor))
      (:CastFailed
        (bind _aslodactor (Utilities|Casting|CastToLODActor _array_element))
        (Networking|SetReplicates _aslodactor true)
        (Actor|DestroyActor _aslodactor)))))

(event Collision|EventActorBeginOverlap
  (params (OtherActor :type Actor%20Object%20Reference))
  (|CallParentFunction OtherActor) ; This node is disabled and will not be called.\nDrag off pins to build functionality.
)

(event EventTick
  (params (DeltaSeconds :type Float%20%28single-precision%29))
  (|CallParentFunction DeltaSeconds) ; This node is disabled and will not be called.\nDrag off pins to build functionality.
)

(fn ConstructionScript
  (|CallParentFunction))