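; Longbow arrow child Blueprint that hooks projectile firing to apply fire arrow and scatter shot behavior.
; On OnProjectileFired it runs the parent logic, then, only if the arrow is not locally predicted, casts its owning controller to BP_SupremacyPlayerController.
; That controller receives the arrow through AssignFireArrowValues and then TryScatterShot, so both effects are delegated to it.
; The construction script only calls the parent, and the other events are disabled stubs.
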(event EventBeginPlay
  (|CallParentFunction) ; This node is disabled and will not be called.\nDrag off pins to build functionality.
)

(event Collision|EventActorBeginOverlap
  (params (OtherActor :type Actor%20Object%20Reference))
  (|CallParentFunction OtherActor) ; This node is disabled and will not be called.\nDrag off pins to build functionality.
)

(event EventTick
  (params (DeltaSeconds :type Float%20%28single-precision%29))
  (|CallParentFunction DeltaSeconds) ; This node is disabled and will not be called.\nDrag off pins to build functionality.
)

(event EventOnProjectileFired
  (bind _self self)
  (|CallParentFunction)
  (if (not (Variables|Default|GetbIsLocallyPredicted))
    (bind _returnvalue (Class|MordhauProjectile|GetProjectileOwningController))
    (bind _asbp_conquest_player_controller (Utilities|Casting|CastToBP_SupremacyPlayerController _returnvalue))
    (Default|AssignFireArrowValues _asbp_conquest_player_controller _self)
    (Default|TryScatterShot _asbp_conquest_player_controller _self)))

(fn ConstructionScript
  (|CallParentFunction))